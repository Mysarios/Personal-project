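; Plus is an addition node Blueprint that sums the values of two linked nodes, as in an expression tree.
; Eval calls Eval on Node1 and Node2, sets its TextRender to the NewVar0 variable rather than the computed sum, and returns the total.
; The event graph holds only disabled default events, and the construction script just calls its parent.
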(fn `Eval`
  (returns (NewParam :type "Float (double-precision)"))
  (locals (NewLocalVar_0 :type "/Game/Project_noods/Eval/АбстрактныеКлассы/NodeEval Object Reference"))
  (bind _newparam (`self.Eval` (`self.Node1`)))
  (bind _newparam_2 (`self.Eval` (`self.Node2`)))
  (`TextRenderComponent.K2_SetText` (`self.TextRender`) (`self.NewVar_0`))
  (return (+ _newparam _newparam_2)))

(fn `UserConstructionScript`
  (`parent.UserConstructionScript`))