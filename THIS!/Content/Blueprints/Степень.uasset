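; Степень ("Power") is an expression node actor that computes a power from two linked nodes and has a text display.
; Eval evaluates Node as the base and Степень as the exponent, truncates the exponent, then repeatedly multiplies Param by the base in a loop.
; It returns Param but sets the TextRender from Value, which this function never assigns.
; The event graph holds only disabled or empty events.
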(event `self.ReceiveActorOnInputTouchEnd`
  (params (FingerIndex :type "ETouchIndex Enum" :default "Touch1")))

(fn `Eval`
  (returns (NewParam :type "Float (double-precision)"))
  (bind _newparam (`self.Eval` (`self.Node`)))
  (bind _newparam_2 (`self.Eval` (`self.Степень`)))
  (for _ (range 1 (+ (`KismetMathLibrary.FTrunc` _newparam_2) 1))
    (set `self.Param` (* _newparam (`self.Param`))))
  (`TextRenderComponent.K2_SetText` (`self.TextRender`) (`self.Value`))
  (return (`self.Param`)))

(fn `UserConstructionScript`
  (`parent.UserConstructionScript`))